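; BP_WallSconce is a wall sconce light with configurable color, brightness, cone angles and lit state.
; Its construction script calls InitializeLight to apply those variables to the SconceLight component, then sets that component's visibility from IsLit.
; TurnLightOn and TurnLightOff are empty stubs, so the file has no logic for switching the light at runtime.
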(fn ConstructionScript
  (CallFunction|InitializeLight)
  (Rendering|SetVisibility (Variables|Default|GetSconceLight) (Variables|Light|GetIsLit) false))

(fn InitializeLight
  (bind _sconcelight (Variables|Default|GetSconceLight))
  (Rendering|Components|Light|SetLightColor _sconcelight (Variables|Light|GetColor) true)
  (Rendering|Lighting|SetInnerConeAngle _sconcelight (Variables|Light|GetInner%20Cone%20Angle))
  (Rendering|Lighting|SetOuterConeAngle _sconcelight (Variables|Light|GetOuter%20Cone%20Angle))
  (Rendering|Components|Light|SetIntensity _sconcelight (Variables|Light|GetBrightness)))

(fn TurnLighton)

(fn TurnLightOff)
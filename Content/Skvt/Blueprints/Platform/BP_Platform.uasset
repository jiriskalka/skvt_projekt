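; A trigger platform that, when its Box is overlapped, sends a Break, Repair, Turn on, Turn Off or Toggle message to nearby electro devices, chosen by Type.
; Devices are gathered from a Radius-sized sphere, and Toggle fires again on end overlap.
; The construction script sizes the sphere and labels the platform with its type in a matching color.
; Each action draws a temporary debug sphere in that color to show its reach.
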(event OnComponentBeginOverlap(Box)
  (params (OverlappedComponent :type Primitive%20Component%20Object%20Reference) (OtherActor :type Actor%20Object%20Reference) (OtherComp :type Primitive%20Component%20Object%20Reference) (OtherBodyIndex :type Integer) (bFromSweep :type Boolean) (SweepResult :type Hit%20Result%20Structure%20%28by%20ref%29))
  (switch Utilities|FlowControl|Switch|SwitchonPlatformTypeEnum (Variables|Default|GetType)
    (:NewEnumerator0
      (CallFunction|Break))
    (:NewEnumerator1
      (CallFunction|Repair))
    (:NewEnumerator2
      (CallFunction|Turnon))
    (:NewEnumerator3
      (CallFunction|TurnOff))
    (:NewEnumerator4
      (CallFunction|Toggle))))

(event OnComponentEndOverlap(Box)
  (params (OverlappedComponent :type Primitive%20Component%20Object%20Reference) (OtherActor :type Actor%20Object%20Reference) (OtherComp :type Primitive%20Component%20Object%20Reference) (OtherBodyIndex :type Integer))
  (if (Utilities|Enum|Equal(Enum) (Variables|Default|GetType) "NewEnumerator4")
    (CallFunction|Toggle)))

(event EventBeginPlay)

(event Collision|EventActorBeginOverlap
  (params (OtherActor :type Actor%20Object%20Reference)))

(event EventTick
  (params (DeltaSeconds :type Float%20%28single-precision%29)))

(fn ConstructionScript
  (Components|Sphere|SetSphereRadius (Variables|Default|GetSphere) (Variables|Default|GetRadius) true)
  (Rendering|Components|TextRender|SetText (Variables|Default|GetTextRender) (Utilities|Text|ToText(String) (Utilities|String|EnumtoString (Variables|Default|GetType))))
  (Rendering|Components|TextRender|SetTextRenderColor (Variables|Default|GetTextRender) (Math|Conversions|ToColor(LinearColor) (CallFunction|GetTypeColor))))

(fn Break
  (CallFunction|ShowAreaOfEffect)
  (for _array_element (CallFunction|GetDevices)
    (Class|BPIElectroDevice|Break(Message) _array_element)))

(fn Repair
  (CallFunction|ShowAreaOfEffect)
  (for _array_element (CallFunction|GetDevices)
    (Class|BPIElectroDevice|Repair(Message) _array_element)))

(fn Toggle
  (CallFunction|ShowAreaOfEffect)
  (for _array_element (CallFunction|GetDevices)
    (Class|BPIElectroDevice|Toggle(Message) _array_element)))

(fn Turnon
  (CallFunction|ShowAreaOfEffect)
  (for _array_element (CallFunction|GetDevices)
    (Class|BPIElectroDevice|Turnon(Message) _array_element)))

(fn TurnOff
  (CallFunction|ShowAreaOfEffect)
  (for _array_element (CallFunction|GetDevices)
    (Class|BPIElectroDevice|TurnOff(Message) _array_element)))

(fn GetDevices
  (bind _overlappingactors (CallFunction|GetElectroDevicesinSphereCollision (Variables|Default|GetSphere)))
  (return _overlappingactors))

(fn ShowAreaOfEffect
  (Rendering|Debug|DrawDebugSphere (Physics|GetCenterOfMass (Variables|Default|GetBox) "None") (Variables|/Script/Engine.SphereComponent|GetSphereRadius (Variables|Default|GetSphere)) 12 (CallFunction|GetTypeColor) 2.0 1.0))

(fn GetTypeColor
  (switch Utilities|FlowControl|Switch|SwitchonPlatformTypeEnum (Variables|Default|GetType)
    (:NewEnumerator0
      (return "(R=0.354167,G=0.066406,B=0.066406,A=1.000000)"))
    (:NewEnumerator1
      (return "(R=0.176674,G=0.588542,B=0.137939,A=1.000000)"))
    (:NewEnumerator2
      (return "(R=0.791667,G=0.602244,B=0.000000,A=1.000000)"))
    (:NewEnumerator3
      (return "(R=0.085341,G=0.124960,B=0.135417,A=1.000000)"))
    (:NewEnumerator4
      (return "(R=0.477749,G=0.221924,B=0.526042,A=1.000000)"))))
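; Player controller that lets the player cycle possession through the pawns in the level.
; On begin play it adds the default and pawn-swap Enhanced Input mapping contexts to the local player subsystem.
; Triggering the swap action gathers all Pawn actors and possesses the one after the currently controlled pawn in that list, wrapping to the first at the end.
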(event Input|EnhancedActionEvents|EnhancedInputActionIA_Swap
  (params (ActionValue :type Boolean) (ElapsedSeconds :type Float%20%28double-precision%29) (TriggeredSeconds :type Float%20%28double-precision%29) (InputAction :type Input%20Action%20Object%20Reference :default "/Game/Skvt/Characters/Input/Actions/IA_Swap.IA_Swap"))
  (:Triggered
    (bind _outactors (Actor|GetAllActorsOfClass "/Script/Engine.Pawn"))
    (Pawn|Possess (CallFunction|GetPawntoPossess _outactors))))

(event EventBeginPlay
  (CallFunction|AddMappingContexts))

(fn ConstructionScript)

(fn AddMappingContexts
  (bind _self self)
  (bind _returnvalue (PlayerController|LocalPlayerSubsystems|GetEnhancedInputLocalPlayerSubsystem _self))
  (Utilities|IsValid _returnvalue
    (:Is%20Valid
      (Input|AddMappingContext _returnvalue "/Game/ThirdPerson/Input/IMC_Default.IMC_Default" 0 "(bIgnoreAllPressedKeysUntilRelease=True,bForceImmediately=False)")
      (Input|AddMappingContext _returnvalue "/Game/Skvt/Characters/Input/IMC_SwapPawn.IMC_SwapPawn" 0 "(bIgnoreAllPressedKeysUntilRelease=True,bForceImmediately=False)"))))

(fn GetPawntoPossess
  (params (PawnAray :type Array%20of%20Pawn%20Object%20References))
  (bind _returnvalue (Pawn|GetControlledPawn))
  (bind _returnvalue_2 (Utilities|Array|FindItem PawnAray _returnvalue))
  (bind _returnvalue_3 (+ _returnvalue_2 1))
  (if (Utilities|Array|IsValidIndex PawnAray _returnvalue_3)
    (return (Utilities|Array|Get(acopy) PawnAray _returnvalue_3))
    (else
      (return (Utilities|Array|Get(acopy) PawnAray)))))